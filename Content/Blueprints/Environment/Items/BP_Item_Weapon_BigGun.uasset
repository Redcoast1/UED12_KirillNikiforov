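; BP_Item_Weapon_BigGun is a weapon pickup item that overrides PutIntoBackpack to hand its weapon to a backpack.
; After the parent call, a valid ItemName is looked up in the backpack's available weapons.
; An owned weapon gets an ammo increase equal to its max rounds, while a new one is added as a weapon item.
; Either way, AfterUse runs afterward; the event graph holds only disabled stubs.
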(fn `PutIntoBackpack`
  (params (InBackpack :type "/Game/Blueprints/Components/BP_BackpackComponent Object Reference"))
  (locals (L_Backpack :type "/Game/Blueprints/Components/BP_BackpackComponent Object Reference"))
  (bind _output_get (set `local.L_Backpack` InBackpack))
  (`parent.PutIntoBackpack` _output_get)
  (if (!= (`self.ItemName`) "None")
    (`|ExecutionSequence`
      (:`then_0`
        (if (`.ReturnValue` (`BlueprintMapLibrary.Map_Find` (`/Game/Blueprints/Components/BP_BackpackComponent.AvalableWeapon` (`local.L_Backpack`)) (`self.ItemName`)))
          (`/Game/Blueprints/Components/BP_BackpackComponent.UpdateAmmoByName` (`local.L_Backpack`) (`self.ItemName`) (`.RoundsMax` (`/Game/Blueprints/Components/BP_BackpackComponent.GetMaxRoundsForWeapon` (`local.L_Backpack`) (`self.ItemName`))) true)
          (else
            (`/Game/Blueprints/Components/BP_BackpackComponent.AddWeaponItem` (`local.L_Backpack`) (`self.ItemName`)))))
      (:`then_1`
        (`self.AfterUse`)))))

(fn `UserConstructionScript`
  (`parent.UserConstructionScript`))