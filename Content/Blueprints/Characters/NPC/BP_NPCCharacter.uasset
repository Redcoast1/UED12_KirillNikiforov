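; Base NPC character Blueprint with a health bar widget and floating text that shows its AI state.
; On BeginPlay it registers itself with the W_HealthBar inside its WidgetHP component.
; Each Tick it checks whether the player pawn is within a fixed range of its capsule.
; When in range, TooltipText displays the BP_AIController's AIState and rotates to face the player's camera.
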(event `self.ReceiveBeginPlay`
  (`parent.ReceiveBeginPlay`)
  (bind _asw_health_bar (cast `/Game/Blueprints/HUD/Widgets/W_HealthBar` (`WidgetComponent.GetUserWidgetObject` (`self.WidgetHP`))))
  (`/Game/Blueprints/HUD/Widgets/W_HealthBar.UpdateCurrentCharacterForHP` _asw_health_bar self))

(event `self.ReceiveTick`
  (params (DeltaSeconds :type "Float (single-precision)"))
  (`parent.ReceiveTick` DeltaSeconds)
  (set `self.IsLookAtPlayerCamera` (<= (`KismetMathLibrary.VSize` (- (`SceneComponent.K2_GetComponentLocation` (`self.CapsuleComponent`)) (`self.K2_GetActorLocation` (`GameplayStatics.GetPlayerPawn` 0)))) 1500.0))
  (`self.LookingAtPlayerCamera`))

(fn `ActionMain`
  (params (IsPressed :type Boolean))
  (`parent.ActionMain` IsPressed))

(fn `LookingAtPlayerCamera`
  (locals (L_CameraLocation :type "Vector Structure" :default (0.0 0.0 0.0)))
  (if (`self.IsLookAtPlayerCamera`)
    (bind _asbp_aicontroller (cast `/Game/Blueprints/Controllers/BP_AIController` (`self.GetController`)))
    ;[1 1 1] Не могу подключить, не разобрался
    (bind _asbp_player_character (cast `/Game/Blueprints/Characters/Player/BP_PlayerCharacter` (`GameplayStatics.GetPlayerPawn` 0)))
    (set `local.L_CameraLocation` (`SceneComponent.K2_GetComponentLocation` (`/Game/Blueprints/Characters/Player/BP_PlayerCharacter.Camera` _asbp_player_character)))
    (`TextRenderComponent.K2_SetText` (`self.TooltipText`) (`|FormatText` " {AIState}" (`|GetEnumeratorNameAsString` (`/Game/Blueprints/Controllers/BP_AIController.AIState` _asbp_aicontroller))))
    (`SceneComponent.K2_SetWorldRotation` (`self.TooltipText`) (`KismetMathLibrary.FindLookAtRotation` (`SceneComponent.K2_GetComponentLocation` (`self.TooltipText`)) (`local.L_CameraLocation`)) false false)))

(fn `UserConstructionScript`
  (`parent.UserConstructionScript`))