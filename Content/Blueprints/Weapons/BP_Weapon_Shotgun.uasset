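; Shotgun weapon Blueprint that fires a horizontal fan of BP_Projectile_Shotgun actors per shot.
; SingleShoot replaces the parent logic, looping up to MaxBulletsInShot to spawn projectiles at MuzzleScene, stepping yaw by ShotAngle, then calls ShotEffects.
; The index offset subtracts MaxBulletsInShot divided by 1, so the fan sits to one side of the muzzle direction instead of centered.
; ConfigureWeaponStats extends the parent with a SetSkeletalMesh call that specifies no mesh.
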(fn `ConfigureWeaponStats`
  (params (InWeaponName :type Name))
  (`parent.ConfigureWeaponStats` InWeaponName)
  (`SkinnedMeshComponent.SetSkinnedAssetAndUpdate` (`self.SkeletalMesh`) null true))

(fn `SingleShoot`
  (locals (L_Index :type Integer))
  (bind (_returnvalue_location _returnvalue_rotation _returnvalue_scale) (`KismetMathLibrary.BreakTransform` (`SceneComponent.K2_GetComponentToWorld` (`self.MuzzleScene`))))
  (`|ExecutionSequence`
    (:`then_0`
      (for _index (range (+ (`self.MaxBulletsInShot`) 1))
        (set `local.L_Index` _index)
        (`|SpawnActorFromClass` "/Game/Blueprints/Weapons/Projectiles/BP_Projectile_Shotgun.BP_Projectile_Shotgun_C" (`KismetMathLibrary.MakeTransform` _returnvalue_location (`KismetMathLibrary.MakeRotator` (.roll _returnvalue_rotation) (.pitch _returnvalue_rotation) (+ (.yaw _returnvalue_rotation) (* (`KismetMathLibrary.Conv_IntToDouble` (- (`local.L_Index`) (/ (`self.MaxBulletsInShot`) 1))) (`self.ShotAngle`)))) _returnvalue_scale) "AdjustIfPossibleButAlwaysSpawn" "OverrideRootScale" self null)))
    (:`then_1`
      (`self.ShotEffects`))))

(fn `UserConstructionScript`
  (`parent.UserConstructionScript`))