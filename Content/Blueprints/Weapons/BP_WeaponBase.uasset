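; Base weapon actor that handles firing, reloading and show/hide on activation, with stats loaded by name from DT_WeaponStats and damage scaled by the owner's stats component.
; While active, Tick polls held fire input through a weapon state machine, with timers for shot delay and reload.
; Shots spawn muzzle FX and type-selected projectiles, with only pistol and rifle classes assigned.
; Reloads draw ammo from the owner's backpack component, or refill fully without one.
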(event `self.ReceiveTick`
  (params (DeltaSeconds :type "Float (single-precision)"))
  (if (`self.IsWeaponActive`)
    (`self.Shooting`)))

(event `/Game/Blueprints/BPI_CustomInterface.ShootProcess`
  (params (InProcess :type Boolean))
  (`self.ShootInputRecived` InProcess))

(fn `ActivateWeapon`
  (params (InActivation :type Boolean))
  (locals (L_StaticMesh :type "Array of StaticMeshComponent Object Reference") (L_SkelMesh :type "Array of SkeletalMeshComponent Object Reference"))
  (set `self.IsWeaponActive` (`local.InActivation`))
  (`|ExecutionSequence`
    (:`then_0`
      (bind _output_get (set `local.L_SkelMesh` (`self.K2_GetComponentsByClass` "/Script/Engine.SkeletalMeshComponent")))
      (if (`KismetArrayLibrary.Array_IsValidIndex` _output_get)
        (for _array_element (`local.L_SkelMesh`)
          (`SceneComponent.SetVisibility` _array_element (`self.IsWeaponActive`) true))))
    (:`then_1`
      (bind _output_get_2 (set `local.L_StaticMesh` (`self.K2_GetComponentsByClass` "/Script/Engine.StaticMeshComponent")))
      (if (`KismetArrayLibrary.Array_IsValidIndex` _output_get_2)
        (for _array_element_2 (`local.L_StaticMesh`)
          (`SceneComponent.SetVisibility` _array_element_2 (`self.IsWeaponActive`) true))))))

(fn `AfterShotDelayEnds`
  (set `self.WeaponState` "NewEnumerator0"))

(fn `ConfigureWeaponStats`
  (params (InWeaponName :type Name))
  (bind _returnvalue (`self.GetOwner`))
  (bind _returnvalue_2 (`self.GetComponentByClass` _returnvalue "/Game/Blueprints/Components/BP_MainStatsComponent.BP_MainStatsComponent_C"))
  (set `self.WeaponName` InWeaponName)
  (if (!= (`self.WeaponName`) "None")
    (bind _returnvalue_3 (`|GetDataTableRow` "/Game/Data/DT_WeaponStats.DT_WeaponStats" (`self.WeaponName`))
      (:`then`
        (set `self.WeaponStats` _returnvalue_3)
        (set `self.RoundsCurrent` (`.RoundsMax_11_E21B4861427F330974C09A8FFC1BF31F` (break `/Game/Blueprints/Structures/STRUCT_WeaponStats` (`self.WeaponStats`))))
        (set `self.DamageCurrent` (`.Damage_20_A2514381479C05FD28AAB9B7F35863C9` (break `/Game/Blueprints/Structures/STRUCT_WeaponStats` (`self.WeaponStats`))))
        (`/Engine/EditorBlueprintResources/StandardMacros.IsValid` _returnvalue
          (:`Is Valid`
            (`/Engine/EditorBlueprintResources/StandardMacros.IsValid` _returnvalue_2
              (:`Is Valid`
                (set `self.DamageCurrent` (`KismetMathLibrary.FTrunc` (* (`self.DamageCurrent`) (`.DamageMult_16_947CC7F44B2D28C518BC2B82A8B569EE` (break `/Game/Blueprints/Structures/STRUCT_MainStats` (`/Game/Blueprints/Components/BP_MainStatsComponent.MainStatsStructure` _returnvalue_2)))))))))))
      (:`RowNotFound`
        (`KismetSystemLibrary.PrintString` "Configure Weapon Sats Failed: Current Name not found in DT" false)))
    (else
      (`KismetSystemLibrary.PrintString` "Configure Weapon Sats Failed: Current Name not found in DT" false))))

(fn `Interact`
  (returns (Success :type Boolean))
  (return false))

(fn `OnReloadDelayEnds`
  (set `self.WeaponState` "NewEnumerator0")
  (`AudioComponent.Play` (`self.ReloadEndSound`) 0.0)
  (`self.OnWeaponStatusChanged`))

(fn `Reaload`
  (bind _returnvalue (`self.GetComponentByClass` (`self.GetOwner`) "/Game/Blueprints/Components/BP_BackpackComponent.BP_BackpackComponent_C"))
  (if (not (`self.In Process`))
    (set `self.WeaponState` "NewEnumerator3")
    (`AudioComponent.Play` (`self.ReloadStartSound`) 0.0)
    (`|ExecutionSequence`
      (:`then_0`
        (`/Engine/EditorBlueprintResources/StandardMacros.IsValid` _returnvalue
          (:`Is Valid`
            (bind _outammo (`/Game/Blueprints/Components/BP_BackpackComponent.UpdateAmmoByName` _returnvalue (`self.WeaponName`) (- (`.RoundsMax_11_E21B4861427F330974C09A8FFC1BF31F` (break `/Game/Blueprints/Structures/STRUCT_WeaponStats` (`self.WeaponStats`))) (`self.RoundsCurrent`)) false))
            (set `self.RoundsCurrent` _outammo))
          (:`Is Not Valid`
            (set `self.RoundsCurrent` (`.RoundsMax_11_E21B4861427F330974C09A8FFC1BF31F` (break `/Game/Blueprints/Structures/STRUCT_WeaponStats` (`self.WeaponStats`)))))))
      (:`then_1`
        (if (!= (`self.RoundsCurrent`) 0)
          (`KismetSystemLibrary.K2_SetTimerDelegate` (`|CreateDelegate` :!event `OnReloadDelayEnds`) (`.ReloadTime_21_B48C5D93400B2CD999A9B29FAC707AFE` (break `/Game/Blueprints/Structures/STRUCT_WeaponStats` (`self.WeaponStats`))))
          (`self.OnWeaponStatusChanged`)
          (else
            (set `self.WeaponState` "NewEnumerator4")
            (`self.OnWeaponStatusChanged`)))))))

(fn `RoundsCount`
  (returns (AllowShooting :type Boolean))
  (bind _result (`/Engine/EditorBlueprintResources/StandardMacros.DecrementInt` (`self.RoundsCurrent`))
    (:`  `
      (return (> _result 0)))))

(fn `Shooting`
  (if (`self.In Process`)
    (if (`|EnumEquality` (`self.WeaponState`) "NewEnumerator0")
      (`self.SingleShoot`)
      (bind _allowshooting (`self.RoundsCount`))
      (if _allowshooting
        (`KismetSystemLibrary.K2_SetTimerDelegate` (`|CreateDelegate` :!event `AfterShotDelayEnds`) (`.ShotTime_17_DC95143248BBFF2D030348BF5169ECBF` (break `/Game/Blueprints/Structures/STRUCT_WeaponStats` (`self.WeaponStats`))))
        (set `self.WeaponState` "NewEnumerator1")
        (`self.OnWeaponStatusChanged`)
        (else
          (set `self.WeaponState` "NewEnumerator2")
          (if (`.AutoReload_24_F0FA4640495975AB2424BDABBD2B9004` (break `/Game/Blueprints/Structures/STRUCT_WeaponStats` (`self.WeaponStats`)))
            (`self.Reaload`)
            (else
              (`self.OnWeaponStatusChanged`)))))
      (else
        (switch `/Game/Blueprints/Enum/ENUM_WeaponState` (`self.WeaponState`)
          (:`NewEnumerator2`
            _)
          (:`NewEnumerator4`
            _))
        (if (not (`AudioComponent.IsPlaying` (`self.MissclickSound`)))
          (`AudioComponent.Play` (`self.MissclickSound`) 0.0))))))

(fn `ShootInputRecived`
  (params (InProcess :type Boolean))
  (set `self.In Process` InProcess))

(fn `ShotEffects`
  (`AudioComponent.Play` (`self.ShootSound`) 0.0)
  (bind _returnvalue (`|SpawnActorFromClass` "/Game/Blueprints/Weapons/Projectiles/BP_MuzzleFX.BP_MuzzleFX_C" (`SceneComponent.K2_GetComponentToWorld` (`self.MuzzleScene`)) "Undefined" "OverrideRootScale" null null))
  (`self.K2_AttachToComponent` _returnvalue (`self.MuzzleScene`) "None" "SnapToTarget" "SnapToTarget" "KeepRelative" true))

(fn `SingleShoot`
  (bind _returnvalue (`|SpawnActorFromClass` (select `/Game/Blueprints/Enum/ENUM_WeaponType` (`.WeaponType_2_9D55D0944E8A68F7495D40BC14F1DB1E` (break `/Game/Blueprints/Structures/STRUCT_WeaponStats` (`self.WeaponStats`))) :`NewEnumerator0` "/Game/Blueprints/Weapons/Projectiles/BP_Projectile_Pistol.BP_Projectile_Pistol_C" :`NewEnumerator1` "/Game/Blueprints/Weapons/Projectiles/BP_Projectile_Rifle.BP_Projectile_Rifle_C" :!type "Actor Class Reference") (`SceneComponent.K2_GetComponentToWorld` (`self.MuzzleScene`)) "Undefined" "OverrideRootScale" self null))
  (cast `/Game/Blueprints/Weapons/Projectiles/BP_ProjectileBase` _returnvalue)
  (`self.ShotEffects`))

(fn `UserConstructionScript`)